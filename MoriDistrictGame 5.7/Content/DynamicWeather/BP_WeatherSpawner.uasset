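; BP_WeatherSpawner is a dynamic weather actor that carries Niagara particles and audio along with the player character.
; On BeginPlay it grabs the player character, and each Tick it eases toward them with VInterpTo at the active weather's follow speed.
; SetWeatherData swaps the particle system, amount, sound and speed when the key changes.
; ClearWeatherData stops effects and fades audio only if its key matches the current one.
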(event EventBeginPlay
  (Variables|Default|SetActorToFollow (Game|GetPlayerCharacter 0)))

(event Collision|EventActorBeginOverlap
  (params (OtherActor :type Actor%20Object%20Reference)))

(event EventTick
  (params (DeltaSeconds :type Float%20%28single-precision%29))
  (bind _actortofollow (Variables|Default|GetActorToFollow))
  (if (Utilities|IsValid _actortofollow)
    (Transformation|SetActorLocation (Math|Interpolation|VInterpTo (Transformation|GetActorLocation) (Transformation|GetActorLocation _actortofollow) DeltaSeconds (Variables|Default|GetFollowingSpeed)) false false)))

(fn ConstructionScript)

(fn SetWeatherData
  (params (WeatherData :type Struc%20F%20Weather%20Data%20Structure))
  (bind _niagara (Variables|Default|GetNiagara))
  (bind _niagara_2 (Variables|Default|GetNiagara))
  (bind _audio (Variables|Default|GetAudio))
  (if (== (Variables|Default|GetCurrentKey) (.key WeatherData))
    (return)
    (else
      (Variables|Default|SetCurrentKey (.key WeatherData))
      (Utilities|FlowControl|Sequence
        (:then_0
          ;[0.15 0.15 0.15 0.5] Particel System Spawning
          (if (Utilities|IsValid (.particlesystem WeatherData))
            (if (Components|Activation|IsActive _niagara_2)
              (Components|Activation|Deactivate _niagara_2))
            (Components|Activation|Activate _niagara_2 false)
            (Class|NiagaraComponent|SetAsset _niagara (.particlesystem WeatherData) true)
            (Niagara|SetNiagaraVariable(Float) _niagara "Amount" (.amount WeatherData))))
        (:then_1
          ;[0.15 0.15 0.15 0.5] Spawn /Add Sound
          (if (Utilities|IsValid (.sound WeatherData))
            (Audio|Components|Audio|SetSound _audio (.sound WeatherData))
            (Audio|Components|Audio|FadeIn _audio 1.0 1.0 0.0 "Linear" :!class /Script/Engine.AudioComponent)))
        (:then_2
          ;[0.15 0.15 0.15 0.5] Set Follow Speed
          (Variables|Default|SetFollowingSpeed (.followingspeed WeatherData)))))))

(fn ClearWeatherData
  (params (Key :type Name))
  (if (== Key (Variables|Default|GetCurrentKey))
    (Variables|Default|SetCurrentKey "None")
    (Components|Activation|Deactivate (Variables|Default|GetNiagara))
    (Variables|Default|SetFollowingSpeed 1.0)
    (Audio|Components|Audio|FadeOut (Variables|Default|GetAudio) 1.0 0.0 "Linear" :!class /Script/Engine.AudioComponent)))