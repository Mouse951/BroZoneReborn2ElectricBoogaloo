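; BP_WeatherOverlapActor is a volume that applies its weather data to a BP_WeatherSpawner that overlaps it.
; Box begin and end overlap events both feed HandleOverlap, which ignores any actor that is not a weather spawner.
; Depending on the overlap type, it either sets the WeatherData on the spawner or clears it by that data's key.
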(event OnComponentBeginOverlap(Box)
  (params (OverlappedComponent :type Primitive%20Component%20Object%20Reference) (OtherActor :type Actor%20Object%20Reference) (OtherComp :type Primitive%20Component%20Object%20Reference) (OtherBodyIndex :type Integer) (bFromSweep :type Boolean) (SweepResult :type Hit%20Result%20Structure%20%28by%20ref%29))
  (CallFunction|HandleOverlap (Variables|Default|GetOnBeginOverlap) OtherActor))

(event OnComponentEndOverlap(Box)
  (params (OverlappedComponent :type Primitive%20Component%20Object%20Reference) (OtherActor :type Actor%20Object%20Reference) (OtherComp :type Primitive%20Component%20Object%20Reference) (OtherBodyIndex :type Integer))
  (CallFunction|HandleOverlap (Variables|Default|GetOnEndOverlap) OtherActor))

(event EventBeginPlay)

(event Collision|EventActorBeginOverlap
  (params (OtherActor :type Actor%20Object%20Reference)))

(event EventTick
  (params (DeltaSeconds :type Float%20%28single-precision%29)))

(fn ConstructionScript)

(fn HandleOverlap
  (params (OverlapType :type Enum_OverlapType%20Enum :default "NewEnumerator0") (OtherActor :type Actor%20Object%20Reference))
  (bind _asbp_weather_spawner (Utilities|Casting|CastToBP_WeatherSpawner OtherActor))
  (switch Utilities|FlowControl|Switch|SwitchonEnum_OverlapType OverlapType
    (:NewEnumerator1
      (Default|SetWeatherData _asbp_weather_spawner (Variables|Default|GetWeatherData)))
    (:NewEnumerator2
      (Default|ClearWeatherData _asbp_weather_spawner (.key (Variables|Default|GetWeatherData))))))