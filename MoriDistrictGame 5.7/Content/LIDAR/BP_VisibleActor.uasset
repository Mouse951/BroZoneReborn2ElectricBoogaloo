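; BP_VisibleActor is an actor in the LIDAR folder that sets the visibility of its static mesh at game start.
; After a short delay on BeginPlay, it checks that the mesh is valid.
; A visible mesh stays shown only if WantVIsible is true and is hidden otherwise, while a mesh that starts hidden is always shown.
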(event EventBeginPlay
  (bind _staticmesh (Variables|Default|GetStaticMesh))
  (Utilities|FlowControl|Delay 0.2)
  (Utilities|IsValid _staticmesh
    (:Is%20Valid
      (if (Rendering|IsVisible _staticmesh)
        (if (Variables|Default|GetWantVIsible?)
          (Rendering|SetVisibility _staticmesh true false :!label _label)
          (else
            (Rendering|SetVisibility (Variables|Default|GetStaticMesh) false false)))
        (else
          (goto _label))))))

(event Collision|EventActorBeginOverlap
  (params (OtherActor :type Actor%20Object%20Reference)))

(event EventTick
  (params (DeltaSeconds :type Float%20%28single-precision%29)))

(fn ConstructionScript)