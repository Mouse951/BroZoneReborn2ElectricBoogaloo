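; BP_Kar is a drivable vehicle pawn that, when possessed by a player, adds its input mappings and equips and runs a child-actor scanner.
; Each tick it averages ground-sensing component hits to set height and tilt, applying drive and turn input through interpolated offsets and rotation rather than physics.
; Pressing E stops its audio, restores the first-person character at the Spawnback point and hands possession back to it.
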(event OnComponentBeginOverlap(enter)
  (params (OverlappedComponent :type Primitive%20Component%20Object%20Reference) (OtherActor :type Actor%20Object%20Reference) (OtherComp :type Primitive%20Component%20Object%20Reference) (OtherBodyIndex :type Integer) (bFromSweep :type Boolean) (SweepResult :type Hit%20Result%20Structure%20%28by%20ref%29))
  ;[0.15 0.15 0.15 0.5] older stuff
  (Utilities|Casting|CastToBP_FirstPersonPlayerController OtherActor)
  (if true
    _))

(event Custom|KharPossesScanner
  (params (NewParam :type Controller%20Object%20Reference))
  ;[0.15 0.15 0.15 0.5] Khar Scanner
  (bind _asplayer_controller (Utilities|Casting|CastToPlayerController NewParam))
  (Variables|Default|SetPlayer%20Controller _asplayer_controller)
  (Input|AddMappingContext (PlayerController|LocalPlayerSubsystems|GetEnhancedInputLocalPlayerSubsystem _asplayer_controller) "/LidarScanner/Input/DemoInput/IMX_DemoInput.IMX_DemoInput" 0 "(bIgnoreAllPressedKeysUntilRelease=True,bForceImmediately=False,bNotifyUserSettings=False)")
  (Utilities|FlowControl|DelayUntilNextTick)
  (bind _asbp_scanner (Utilities|Casting|CastToBP_Scanner (Variables|/Script/Engine.ChildActorComponent|GetChildActor (Variables|Default|GetChildActor))))
  (Default|Equip _asbp_scanner)
  (Variables|/LidarScanner/BP_Scanner.BP_Scanner_C|SetRunScan _asbp_scanner true))

(event Custom|stopKar
  (Audio|Components|Audio|Stop (Variables|Default|GetIdle))
  (Audio|Components|Audio|Stop (Variables|Default|GetMoving)))

(event Input|EnhancedActionEvents|EnhancedInputActionIA_Drive
  (params (ActionValue :type Float%20%28double-precision%29) (ElapsedSeconds :type Float%20%28double-precision%29) (TriggeredSeconds :type Float%20%28double-precision%29) (InputAction :type Input%20Action%20Object%20Reference :default "/Game/Inputs/IA_Drive.IA_Drive"))
  (:Triggered
    (Variables|Default|SetTargetForwardSpeed (* ActionValue (Variables|Default|GetMaxForwardSpeed))))
  (:Completed
    (Variables|Default|SetTargetForwardSpeed 0.0)))

(event Input|EnhancedActionEvents|EnhancedInputActionIA_Turn
  (params (ActionValue :type Float%20%28double-precision%29) (ElapsedSeconds :type Float%20%28double-precision%29) (TriggeredSeconds :type Float%20%28double-precision%29) (InputAction :type Input%20Action%20Object%20Reference :default "/Game/Inputs/IA_Turn.IA_Turn"))
  (:Triggered
    (Variables|Default|SetTargetTurnSpeed (* ActionValue (Variables|Default|GetMaxTurnSpeed))))
  (:Completed
    (Variables|Default|SetTargetTurnSpeed 0.0)))

(event Input|EnhancedActionEvents|EnhancedInputActionIA_Scan
  (params (ActionValue :type Boolean) (ElapsedSeconds :type Float%20%28double-precision%29) (TriggeredSeconds :type Float%20%28double-precision%29) (InputAction :type Input%20Action%20Object%20Reference :default "/Game/LIDAR/Inputs/IA_Scan.IA_Scan"))
  ;[0.15 0.15 0.15 0.5] older stuff
)

(event EventBeginPlay
  ;[0.15 0.15 0.15 0.5] Begin Play
  (Class|PrimitiveComponent|SetVisibleinSceneCaptureOnly (Variables|Default|GetfakeKar) true)
  (Variables|Default|SetGroundSensingArraay (Actor|GetComponentsByClass "/Game/Kar_bp/BP_GroundSensing.BP_GroundSensing_C"))
  (Audio|Components|Audio|Stop (Variables|Default|GetMoving))
  (Audio|Components|Audio|Stop (Variables|Default|GetIdle)))

(event EventTick
  (params (DeltaSeconds :type Float%20%28single-precision%29))
  (bind _returnvalue (Utilities|Time|GetWorldDeltaSeconds))
  (bind _returnvalue_2 (Utilities|Time|GetWorldDeltaSeconds))
  (Utilities|FlowControl|Sequence
    (:then_0
      (Variables|Default|SetCountOnGround 0)
      (Variables|Default|SetAverageHeight 0.0)
      (Variables|Default|SetAverageNormal "0, 0, 0")
      (for _array_element (Variables|Default|GetGroundSensingArraay)
        (Variables|Default|SetAverageNormal (+ (Variables|/Game/Kar_bp/BP_GroundSensing.BP_GroundSensing_C|GetHitNormal _array_element) (Variables|Default|GetAverageNormal)))
        (Variables|Default|SetAverageHeight (+ (.z (Variables|/Game/Kar_bp/BP_GroundSensing.BP_GroundSensing_C|GethitLocation _array_element)) (Variables|Default|GetAverageHeight)))
        (if (Variables|/Game/Kar_bp/BP_GroundSensing.BP_GroundSensing_C|GetbOnGround _array_element)
          (Math|Integer|IncrementInt (Variables|Default|GetCountOnGround))))
      (Variables|Default|SetAverageNormal (/ (Variables|Default|GetAverageNormal) (Variables|Default|GetCountOnGround)))
      (bind _output_get (Variables|Default|SetAverageHeight (/ (Variables|Default|GetAverageHeight) (Variables|Default|GetCountOnGround))))
      (Variables|Default|SetDeltaZ (- (+ _output_get (Variables|Default|GetHeightOffset)) (.z (Transformation|GetActorLocation))))
      (Transformation|SetActorRotation (Math|Interpolation|RInterpTo (Transformation|GetActorRotation) (Math|Rotator|CombineRotators (Math|Rotator|MakeRotator 0.0 0.0 (* (Variables|Default|GetTargetTurnSpeed) _returnvalue_2)) (Math|Rotator|MakeRotfromZY (Variables|Default|GetAverageNormal) (Transformation|GetActorRightVector))) _returnvalue_2 8.0))
      (Transformation|AddActorWorldOffset (+ (* (Transformation|GetActorForwardVector) (Math|Interpolation|FInterpTo (Variables|Default|GetCurrentForwardSpeed) (Variables|Default|GetTargetForwardSpeed) _returnvalue 2.0) _returnvalue) (* (Transformation|GetActorUpVector) (Variables|Default|GetDeltaZ))))
      (Variables|Default|SetCurrentForwardSpeed (Math|Interpolation|FInterpTo (Variables|Default|GetCurrentForwardSpeed) (Variables|Default|GetTargetForwardSpeed) _returnvalue 2.0)))
    (:then_1
      (if (or (> (Variables|Default|GetCurrentForwardSpeed) 0.0) (> (Variables|Default|GetTargetTurnSpeed) 0.0))
        _))))

(event EventPossessed
  (params (NewController :type Controller%20Object%20Reference))
  ;[0.15 0.15 0.15 0.5] Possession events
  (if (Class|Controller|IsPlayerController NewController)
    (Input|AddMappingContext (PlayerController|LocalPlayerSubsystems|GetEnhancedInputLocalPlayerSubsystem (Game|GetPlayerController 0)) "/Game/Inputs/IMC_Kar.IMC_Kar" 1 "(bIgnoreAllPressedKeysUntilRelease=True,bForceImmediately=False,bNotifyUserSettings=False)")
    (CallFunction|KharPossesScanner NewController)))

(event EventUnpossessed
  (params (OldController :type Controller%20Object%20Reference))
  (bind _returnvalue (Game|GetPlayerController 0))
  (bind _returnvalue_2 (PlayerController|LocalPlayerSubsystems|GetEnhancedInputLocalPlayerSubsystem _returnvalue))
  ;[0.15 0.15 0.15 0.5] Possession events
  (if (and (Class|Controller|IsPlayerController (stale EventPossessed NewController)) (.ReturnValue (Class|EnhancedInputSubsystemInterface|HasMappingContext _returnvalue_2 "/Game/Inputs/IMC_Kar.IMC_Kar")))
    (Input|RemoveMappingContext _returnvalue_2 "/Game/Inputs/IMC_Kar.IMC_Kar" "(bIgnoreAllPressedKeysUntilRelease=True,bForceImmediately=False,bNotifyUserSettings=False)")))

(event Input|KeyboardEvents|E
  (params (Key :type Key%20Structure :default "None"))
  (bind _spawnback (Variables|Default|Getspawnback))
  (bind _returnvalue (Transformation|GetWorldTransform _spawnback))
  (:Pressed
    (Variables|Default|Setdrive false)
    (bind _returnvalue_2 (Actor|GetActorOfClass "/Game/FirstPerson/Blueprints/BP_FirstPersonCharacter.BP_FirstPersonCharacter_C"))
    (Rendering|SetActorHiddenInGame _returnvalue_2 false)
    (Transformation|SetActorTransform _returnvalue_2 (Math|Transform|MakeTransform (.location _returnvalue) (.rotation _returnvalue) "1.000000,1.000000,1.000000"))
    (CallFunction|StopKar)
    (Pawn|Possess (Game|GetPlayerController 0) _returnvalue_2)))

(fn ConstructionScript)